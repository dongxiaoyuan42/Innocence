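; BP_Wall is a wall actor tied to BP_Boss that carries the player until it meets a transport-tagged actor.
; On BeginPlay it requires a BP_Boss instigator, spawns BP_Transport at that boss mesh's EndOfWall socket, then attaches the player pawn to itself, keeping world transform.
; Its Box overlap destroys the wall when the other actor has the Transport tag; no movement logic appears in its graphs.
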(event `self.ReceiveBeginPlay`
  (bind _asbp_boss (cast `/Game/AI/BP_Boss` (`self.GetInstigator`)))
  (`|SpawnActorFromClass` "/Game/AI/BluePrints/BP_Transport.BP_Transport_C" (`SceneComponent.GetSocketTransform` (`Character.Mesh` _asbp_boss) "EndOfWall" "RTS_World") "Undefined" "OverrideRootScale" null null)
  (bind _output_get (set `self.Player` (`GameplayStatics.GetPlayerPawn` 0)))
  (`self.K2_AttachToActor` _output_get self "None" "KeepWorld" "KeepWorld" "KeepWorld" false))

(event `self.Box.OnComponentBeginOverlap`
  (params (OverlappedComponent :type "PrimitiveComponent Object Reference") (OtherActor :type "Actor Object Reference") (OtherComp :type "PrimitiveComponent Object Reference") (OtherBodyIndex :type Integer) (bFromSweep :type Boolean) (SweepResult :type "HitResult Structure (by ref)"))
  (if (`self.ActorHasTag` OtherActor "Transport")
    (`self.K2_DestroyActor`)))

(fn `UserConstructionScript`)